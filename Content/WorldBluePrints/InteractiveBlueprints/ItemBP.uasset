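; ItemBP is an interactive pickup actor that feeds a Poor character when hit.
; It applies its NewMesh to the mesh on BeginPlay.
; IsHit casts the passed character: a Poor gains Hunger, and the item destroys itself and plays an eating sound at its location.
; A Rich character is only cast and validity-checked, as its Social gain, destroy and sound logic is left unconnected.
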(event `self.ReceiveBeginPlay`
  (`StaticMeshComponent.SetStaticMesh` (`self.Mesh`) (`self.NewMesh`)))

(event `IsHit`
  (params (`Character Reference` :type "/Game/Character/CharacterFeelingsBP Object Reference"))
  ;[0.2261 0 1] Item Functionality
  (bind _aspoor (cast `/Game/Character/Poor` `Character Reference`)
    (:`then`
      (`/Engine/EditorBlueprintResources/StandardMacros.IsValid` _aspoor
        (:`Is Valid`
          (bind _output_get (set `/Game/Character/Poor.Hunger` (+ (stale _output_get) 10.0) _aspoor))
          (`self.K2_DestroyActor`)
          (`GameplayStatics.PlaySoundAtLocation` (`self.EatingSound`) (`self.K2_GetActorLocation`) (struct) 1.0 1.0 0.0 null null null))))
    (:`CastFailed`
      (bind _asrich (cast `/Game/Character/Rich` `Character Reference`))
      (`/Engine/EditorBlueprintResources/StandardMacros.IsValid` _asrich))))

(fn `UserConstructionScript`)